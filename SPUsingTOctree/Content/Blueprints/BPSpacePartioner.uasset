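; Demo space partitioner Blueprint that exercises an octree on BeginPlay.
; It initializes a bounded octree, spawns about twenty OctreeDemoElement actors at seeded random positions, and registers each with its Cube component's bounds.
; It then runs two hard-coded box queries with persistent debug drawing and prints the names of the actors found.
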(event `self.ReceiveBeginPlay`
  (bind _randstream (`self.RandStream`))
  (`|ExecutionSequence`
    (:`then_0`
      ;[1 1 1] Initialize Octree
      (`self.Initialize` (`KismetMathLibrary.MakeBox` (-1000.0 -1000.0 -1000.0) (1000.0 1000.0 1000.0)) (`self.DrawDebugInfo`))
      (for _ (range (+ (`KismetMathLibrary.RandomIntegerInRangeFromStream` 20 21 _randstream) 1))
        (bind _returnvalue (`|SpawnActorFromClass` "/Game/Blueprints/OctreeDemoElement.OctreeDemoElement_C" (`KismetMathLibrary.MakeTransform` (`KismetMathLibrary.MakeVector` (`KismetMathLibrary.RandomFloatInRangeFromStream` -1000.0 1000.0 _randstream) (`KismetMathLibrary.RandomFloatInRangeFromStream` -1000.0 1000.0 _randstream) (`KismetMathLibrary.RandomFloatInRangeFromStream` -1000.0 1000.0 _randstream))) "AdjustIfPossibleButDontSpawnIfColliding" "OverrideRootScale" null null))
        (bind (_origin _boxextent _sphereradius) (`KismetSystemLibrary.GetComponentBounds` (`/Game/Blueprints/OctreeDemoElement.Cube` _returnvalue)))
        (`self.AddOctreeElement` (make `OctreeElement` _returnvalue (`KismetMathLibrary.MakeBoxSphereBounds` _origin _boxextent _sphereradius)))))
    (:`then_1`
      (bind _returnvalue_2 (`self.GetElementsWithinBounds` (`KismetMathLibrary.MakeBoxSphereBounds` (-355.130432 -580.99176 -868.926025) (50.0 50.0 50.0) 50.0) true true))
      (for _array_element _returnvalue_2
        (`KismetSystemLibrary.PrintString` (`KismetSystemLibrary.GetDisplayName` (break `OctreeElement` _array_element)) true true (struct :`R` 1.0 :`G` 0.939944 :`B` 0.023497 :`A` 1.0) 10.0))
      (bind _returnvalue_3 (`self.GetElementsWithinBounds` (`KismetMathLibrary.MakeBoxSphereBounds` (-600.0 -400.0 0.0) (150.0 150.0 150.0) 150.0) true true))
      (for _array_element_2 _returnvalue_3
        (`KismetSystemLibrary.PrintString` (`KismetSystemLibrary.GetDisplayName` (break `OctreeElement` _array_element_2)) true true (struct :`R` 1.0 :`G` 0.057804 :`A` 1.0) 10.0)))))

(fn `UserConstructionScript`)